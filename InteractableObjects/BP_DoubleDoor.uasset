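; BP_DoubleDoor is an interactable double fire door that toggles open and closed.
; The Interact event switches on a Status variable, flips it and plays the matching open or close sound at the door's location.
; The DoorMechanics timeline plays forward to open and reverses to close, with separate yaw tracks rotating each of the two door meshes.
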(event `self.Interact`
  ;[1 1 1] Interact with Fire Door
  (switch `/Game/InteractableObjects/EN_DoorStatus` (`self.Status`)
    (:`NewEnumerator0`
      (`GameplayStatics.PlaySoundAtLocation` "/Game/Audio/open-door-sound-247415-_AudioTrimmer_com_.open-door-sound-247415-_AudioTrimmer_com_" (`self.K2_GetActorLocation`) (struct) 1.0 1.0 0.0 null null null null)
      (set `self.Status` "NewEnumerator1")
      (bind (_direction _door_z_rotation _2nddoor) (`Timeline|DoorMechanics` :`NewTime` 2.0 :!label _label)
        (:`Update`
          (`|ExecutionSequence`
            (:`then_0`
              (`SceneComponent.K2_SetRelativeRotation` (`self.StaticMesh`) (`KismetMathLibrary.MakeRotator` 0.0 0.0 _door_z_rotation) false false))
            (:`then_1`
              (`SceneComponent.K2_SetRelativeRotation` (`self.StaticMesh1`) (`KismetMathLibrary.MakeRotator` 0.0 0.0 _2nddoor) false false))))))
    (:`NewEnumerator1`
      (`GameplayStatics.PlaySoundAtLocation` "/Game/Audio/close-door-sound-247450-_AudioTrimmer_com_.close-door-sound-247450-_AudioTrimmer_com_" (`self.K2_GetActorLocation`) (struct) 1.0 1.0 0.0 null null null null)
      (set `self.Status` "NewEnumerator0")
      (goto _label :!via `Reverse`))))

(fn `UserConstructionScript`)