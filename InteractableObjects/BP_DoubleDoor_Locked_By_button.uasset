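; Interactable double door that stays locked until the first-person character overlaps its Box component, which unlocks it with no relock.
; Interact toggles a Status between Closed and Open, playing or reversing one timeline that drives the yaw of both door meshes through separate tracks.
; Closing plays a door sound, and interacting while locked plays a switch sound instead of moving the doors.
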(event `self.Interact`
  ;[1 1 1] Interact with Fire Door
  (if (`self.Unlocked`)
    (switch `/Game/InteractableObjects/EN_DoorStatus` (`self.Status`)
      (:`NewEnumerator0`
        (set `self.Status` "NewEnumerator1")
        (bind (_direction _door_z_rotation _2nddoor) (`Timeline|Timeline_0` :`NewTime` 2.0 :!label _label)
          (:`Update`
            (`|ExecutionSequence`
              (:`then_0`
                (`SceneComponent.K2_SetRelativeRotation` (`self.StaticMesh`) (`KismetMathLibrary.MakeRotator` 0.0 0.0 _door_z_rotation) false false))
              (:`then_1`
                (`SceneComponent.K2_SetRelativeRotation` (`self.StaticMesh1`) (`KismetMathLibrary.MakeRotator` 0.0 0.0 _2nddoor) false false))))))
      (:`NewEnumerator1`
        (`GameplayStatics.PlaySoundAtLocation` "/Game/Audio/close-door-sound-247450-_AudioTrimmer_com_.close-door-sound-247450-_AudioTrimmer_com_" (`self.K2_GetActorLocation`) (struct) 1.0 1.0 0.0 null null null null)
        (set `self.Status` "NewEnumerator0")
        (goto _label :!via `Reverse`)))
    (else
      (`GameplayStatics.PlaySoundAtLocation` "/Engine/VREditor/Sounds/UI/Flashlight_Switch.Flashlight_Switch" (`self.K2_GetActorLocation`) (struct) 1.0 1.0 0.0 null null null null))))

(event `self.Box.OnComponentBeginOverlap`
  (params (OverlappedComponent :type "PrimitiveComponent Object Reference") (OtherActor :type "Actor Object Reference") (OtherComp :type "PrimitiveComponent Object Reference") (OtherBodyIndex :type Integer) (bFromSweep :type Boolean) (SweepResult :type "HitResult Structure (by ref)"))
  ;[1 1 1] Interact with Fire Door
  (cast `/Game/FirstPerson/Blueprints/BP_FirstPersonCharacter` OtherActor)
  (set `self.Unlocked` true))

(fn `UserConstructionScript`)