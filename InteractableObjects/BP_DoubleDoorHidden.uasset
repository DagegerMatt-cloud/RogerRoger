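; BP_DoubleDoorHidden is an interactable double door that swings open or closed on each Interact event.
; A Status value selects whether the DoorMechanics timeline plays or reverses, with its two tracks driving the relative yaw of the two static meshes.
; Each timeline update also plays a dirt footstep sound under HitDoor concurrency, at a location converted from the rotation float rather than the door's position.
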(event `self.Interact`
  ;[1 1 1] Interact with Fire Door
  (switch `/Game/InteractableObjects/EN_DoorStatus` (`self.Status`)
    (:`NewEnumerator0`
      (set `self.Status` "NewEnumerator1")
      (bind (_direction _door_z_rotation _2nddoor) (`Timeline|DoorMechanics` :`NewTime` 2.0 :!label _label)
        (:`Update`
          (`|ExecutionSequence`
            (:`then_0`
              (`SceneComponent.K2_SetRelativeRotation` (`self.StaticMesh`) (`KismetMathLibrary.MakeRotator` 0.0 0.0 _door_z_rotation) false false)
              (`GameplayStatics.PlaySoundAtLocation` "/Game/ProceduralBuildingGenerator/Sound/Wav/Footstep_Dirt02.Footstep_Dirt02" (`KismetMathLibrary.Conv_DoubleToVector` _door_z_rotation) (struct) 1.0 1.0 0.0 null "/Game/Audio/HitDoor.HitDoor" null null))
            (:`then_1`
              (`SceneComponent.K2_SetRelativeRotation` (`self.StaticMesh1`) (`KismetMathLibrary.MakeRotator` 0.0 0.0 _2nddoor) false false))))))
    (:`NewEnumerator1`
      (set `self.Status` "NewEnumerator0")
      (goto _label :!via `Reverse`))))

(fn `UserConstructionScript`)