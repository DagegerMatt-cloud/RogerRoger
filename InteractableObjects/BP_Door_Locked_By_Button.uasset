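; Interactable door Blueprint that opens and closes on Interact only while its Unlocked flag is set, otherwise playing a switch sound.
; A Status value toggles the door, playing open or close sounds and running a Timeline forward or in reverse to drive door yaw.
; The Construction Script uses DoorMode to show or hide the right door, which rotates on its own Timeline track when visible.
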(event `self.Interact`
  ;[1 1 1] Interact with Locked-- Door
  (if (`self.Unlocked`)
    (switch `/Game/InteractableObjects/EN_DoorStatus` (`self.Status`)
      (:`NewEnumerator0`
        (`GameplayStatics.PlaySoundAtLocation` "/Game/Audio/open-door-sound-247415-_AudioTrimmer_com_.open-door-sound-247415-_AudioTrimmer_com_" (`self.K2_GetActorLocation`) (struct) 1.0 1.0 0.0 null null null null)
        (set `self.Status` "NewEnumerator1")
        (bind (_direction _door_z_rotation _2nddoor) (`Timeline|Timeline` :`NewTime` 2.0 :!label _label)
          (:`Update`
            (if (`SceneComponent.IsVisible` (`self.RightDoor`))
              (`|ExecutionSequence`
                (:`then_0`
                  (`SceneComponent.K2_SetRelativeRotation` (`self.LeftDoor`) (`KismetMathLibrary.MakeRotator` 0.0 0.0 _door_z_rotation) false false :!label _label_2))
                (:`then_1`
                  (`SceneComponent.K2_SetRelativeRotation` (`self.RightDoor`) (`KismetMathLibrary.MakeRotator` 0.0 0.0 _2nddoor) false false)))
              (else
                (goto _label_2))))))
      (:`NewEnumerator1`
        (`GameplayStatics.PlaySoundAtLocation` "/Game/Audio/close-door-sound-247450-_AudioTrimmer_com_.close-door-sound-247450-_AudioTrimmer_com_" (`self.K2_GetActorLocation`) (struct) 1.0 1.0 0.0 null null null null)
        (set `self.Status` "NewEnumerator0")
        (goto _label :!via `Reverse`)))
    (else
      (`GameplayStatics.PlaySoundAtLocation` "/Engine/VREditor/Sounds/UI/Flashlight_Switch.Flashlight_Switch" (`self.K2_GetActorLocation`) (struct) 1.0 1.0 0.0 null null null null))))

(fn `UserConstructionScript`
  (bind _rightdoor (`self.RightDoor`))
  (switch `/Game/InteractableObjects/DoorConfig` (`self.DoorMode`)
    (:`NewEnumerator0`
      (`SceneComponent.SetVisibility` _rightdoor false false))
    (:`NewEnumerator1`
      (`SceneComponent.SetVisibility` _rightdoor true false)
      (`PrimitiveComponent.SetCollisionEnabled` _rightdoor "QueryAndPhysics"))))